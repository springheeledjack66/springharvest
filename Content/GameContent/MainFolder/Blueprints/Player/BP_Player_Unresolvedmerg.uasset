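; Player Blueprint with camera-relative movement and a basic melee attack, starting with the "None" weapon.
; Attack input calls the stamina component, then runs a debug-drawn box overlap in front of the player for Pawns.
; Overlapped actors implementing BpInterface_Damageable get a ChangeHealth message with a zero value.
; The player's own ChangeHealth event only prints a string, and its ChangeStamina event is empty.
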(event `InputAction|Attack`
  (params (Key :type "Key Structure"))
  (bind _box_extent (`self.Box Extent`))
  (bind _returnvalue (+ (* (`self.GetActorForwardVector`) (`self.attackDistance`)) (`self.K2_GetActorLocation`)))
  (:`Pressed`
    ;[1 1 1] Enemy AttackingLogic
    (`/Game/GameContent/MainFolder/Blueprints/Components/BP_StaminaComponent.ChangeStamina` (`self.BP_StaminaComponent`))
    (`KismetSystemLibrary.DrawDebugBox` _returnvalue _box_extent (struct :`R` 0.255 :`G` 0.057691 :`B` 0.04754 :`A` 1.0) (`self.K2_GetActorRotation`) 3.0 5.0)
    (bind (_outactors _returnvalue_2) (`KismetSystemLibrary.BoxOverlapActors` _returnvalue _box_extent (`|MakeArray` "ObjectTypeQuery3" :!type "EObjectTypeQuery Enum") "/Script/Engine.Actor" (`|MakeArray` self :!type "Actor Object Reference")))
    (if _returnvalue_2
      (for _array_element _outactors
        (if (`KismetSystemLibrary.DoesImplementInterface` _array_element "/Game/GameContent/MainFolder/Blueprints/BpInterface_Damageable.BpInterface_Damageable_C")
          (message `/Game/GameContent/MainFolder/Blueprints/BpInterface_Damageable.ChangeHealth` _array_element 0.0))))))

(event `self.ReceiveBeginPlay`
  ;[1 1 1] Begin play and set weapon
  (`ActorComponent.Activate` (`self.Camera1`) false)
  (`/Game/GameContent/MainFolder/Blueprints/Components/BP_WeaponComponent.ChangeWeapon` (`self.BP_WeaponComponent`) "None"))

(event `InputAxis|MoveForward`
  (params (AxisValue :type "Float (single-precision)"))
  (`self.AddMovementInput` (`SceneComponent.GetForwardVector` (`self.Camera1`)) AxisValue))

(event `InputAxis|MoveRight`
  (params (AxisValue :type "Float (single-precision)"))
  (`self.AddMovementInput` (`SceneComponent.GetRightVector` (`self.Camera1`)) AxisValue))

(event `/Game/GameContent/MainFolder/Blueprints/BpInterface_Damageable.ChangeHealth`
  (params (Amount :type "Float (double-precision)"))
  (`KismetSystemLibrary.PrintString` "taking damage"))

(event `/Game/GameContent/MainFolder/Blueprints/BPInterface_Stamina.ChangeStamina`
  (params (Amount :type "Float (double-precision)")))

(fn `UserConstructionScript`)