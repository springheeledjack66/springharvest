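; Template pickup actor that the player collects into an inventory and later uses to add health and stamina.
; Trigger overlap toggles a prompt widget and in-range flag, gating a handler bound to the player's PickupItem dispatcher.
; Pickup adds the item struct, with a self-reference, to the inventory, refreshes the HUD and hides the actor without collision.
; The hidden actor persists until UseAction applies its stat bonuses and destroys it.
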(event `self.ReceiveBeginPlay`
  (bind _iteminfo (`self.ItemInfo`))
  (bind _pickuptextreference (`self.PickupTextReference`))
  (bind (_item _itemimage _pickuptext) (break `/Game/Avo_Blueprints/InventoryStructure` _iteminfo))
  ;[1 1 1] Event Begin Play
  (bind _returnvalue (`|CreateWidget` "/Game/Avo_Blueprints/PickUpText.PickUpText_C"))
  (set `self.PickupTextReference` _returnvalue)
  (setmembers `/Game/Avo_Blueprints/InventoryStructure` :`StructRef` _iteminfo :`Item` self)
  (set `/Game/Avo_Blueprints/PickUpText.PickupActor` _item _pickuptextreference)
  (set `/Game/Avo_Blueprints/PickUpText.PickupText` _pickuptext _pickuptextreference)
  (bind _asbp_player (cast `/Game/GameContent/MainFolder/Blueprints/Player/BP_Player` (`GameplayStatics.GetPlayerCharacter` 0)))
  (bind _output_get (set `self.CharacterReference` _asbp_player))
  (add `/Game/GameContent/MainFolder/Blueprints/Player/BP_Player.PickupItem` _output_get (delegate `PickupItem_Event_0`)))

(event `self.Trigger.OnComponentBeginOverlap`
  (params (OverlappedComponent :type "PrimitiveComponent Object Reference") (OtherActor :type "Actor Object Reference") (OtherComp :type "PrimitiveComponent Object Reference") (OtherBodyIndex :type Integer) (bFromSweep :type Boolean) (SweepResult :type "HitResult Structure (by ref)"))
  ;[1 1 1] Overlap Trigger Script
  (cast `/Game/GameContent/MainFolder/Blueprints/Player/BP_Player` OtherActor)
  (`UserWidget.AddToViewport` (`self.PickupTextReference`) 0)
  (set `self.IsInRange` true))

(event `PickupItem_Event_0`
  (bind _characterreference (`self.CharacterReference`))
  ;[1 1 1] Pickup and Add Items to Inventory
  (if (and (`self.GetActorEnableCollision`) (`self.IsInRange`))
    (`KismetArrayLibrary.Array_Add` (`/Game/GameContent/MainFolder/Blueprints/Player/BP_Player.Inventory` _characterreference) (`self.ItemInfo`))
    (`Widget.RemoveFromParent` (`self.PickupTextReference`))
    (`self.SetActorHiddenInGame` true)
    (`self.SetActorEnableCollision` false)
    (`/Game/Avo_Blueprints/PlayerHUD.RefreshInventory` (`/Game/GameContent/MainFolder/Blueprints/Player/BP_Player.GameHUD Reference` _characterreference))))

(event `self.Trigger.OnComponentEndOverlap`
  (params (OverlappedComponent :type "PrimitiveComponent Object Reference") (OtherActor :type "Actor Object Reference") (OtherComp :type "PrimitiveComponent Object Reference") (OtherBodyIndex :type Integer))
  ;[1 1 1] Overlap Trigger Script
  (cast `/Game/GameContent/MainFolder/Blueprints/Player/BP_Player` OtherActor)
  (`Widget.RemoveFromParent` (`self.PickupTextReference`))
  (set `self.IsInRange` false))

(event `/Game/Avo_Blueprints/ActionInterface.UseAction`
  (bind _characterreference (`self.CharacterReference`))
  ;[1 1 1] Use Item
  (set `/Game/GameContent/MainFolder/Blueprints/Player/BP_Player.HealthValue` (+ (`/Game/GameContent/MainFolder/Blueprints/Player/BP_Player.HealthValue` _characterreference) (`self.AddHealth`)) _characterreference)
  (set `/Game/GameContent/MainFolder/Blueprints/Player/BP_Player.StaminaValue` (+ (`/Game/GameContent/MainFolder/Blueprints/Player/BP_Player.StaminaValue` _characterreference) (`self.AddStamina`)) _characterreference)
  (`self.K2_DestroyActor`))

(fn `UserConstructionScript`)